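; Enemy AI controller that runs BT_Enemy and feeds its blackboard from perception and damage events.
; Seeing the third-person character sets TargetActor; losing sight clears it and stores the character's current position as TargetLocation and LastSeenLocation.
; Any other sense, treated as noise, sets TargetLocation to a random reachable point around the stimulus.
; Damage to its Instigator pawn makes the damage causer the TargetActor.
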(event OnTargetPerceptionUpdated(AIPerception)
  (params (Actor :type Actor%20Object%20Reference) (Stimulus :type AI%20Stimulus%20Structure))
  (bind _returnvalue (AI|GetBlackboard 0))
  (bind _returnvalue_2 (Utilities|Name|MakeLiteralName "TargetActor"))
  (bind _returnvalue_3 (Class|AIPerceptionSystem|GetSenseClassforStimulus Stimulus))
  (if (== _returnvalue_3 "/Script/AIModule.AISense_Sight")
    (bind _info (Class|AIPerceptionComponent|GetActorsPerception (Variables|Default|GetAIPerception) Actor))
    (bind _asbp_third_person_character (Utilities|Casting|CastToBP_ThirdPersonCharacter Actor))
    (if (.bSuccessfullySensed (Utilities|Struct|BreakAIStimulus (Utilities|Array|Get(acopy) (.LastSensedStimuli (Utilities|Struct|BreakActorPerceptionBlueprintInfo _info)))))
      (AI|Components|Blackboard|SetValueasObject _returnvalue _returnvalue_2 _asbp_third_person_character)
      (else
        (bind _output_get (Variables|Default|SetLastSensedLocation (Transformation|GetActorLocation _asbp_third_person_character)))
        (AI|Components|Blackboard|SetValueasObject _returnvalue _returnvalue_2 0)
        (AI|Components|Blackboard|SetValueasVector _returnvalue (Utilities|Name|MakeLiteralName "TargetLocation") _output_get)
        (AI|Components|Blackboard|SetValueasVector _returnvalue (Utilities|Name|MakeLiteralName "LastSeenLocation") _output_get)))
    (else
      ;[1 1 1] Noise part of the AI
      (AI|Components|Blackboard|SetValueasVector (AI|GetBlackboard 0) (Utilities|Name|MakeLiteralName "TargetLocation") (.RandomLocation (AI|Navigation|GetRandomReachablePointinRadius (.StimulusLocation (Utilities|Struct|BreakAIStimulus Stimulus)) 1e+03 0 0))))))

(event Custom|TakeDamage
  (params (DamagedActor :type Actor%20Object%20Reference) (Damage :type Float%20%28single-precision%29) (DamageType :type Damage%20Type%20Object%20Reference) (InstigatedBy :type Controller%20Object%20Reference) (DamageCauser :type Actor%20Object%20Reference))
  ;[1 1 1] Follow after take damage
  (AI|Components|Blackboard|SetValueasObject (AI|GetBlackboard 0) (Utilities|Name|MakeLiteralName "TargetActor") DamageCauser))

(event EventBeginPlay
  (AI|RunBehaviorTree "/Game/Blueprints/BT_Enemy.BT_Enemy")
  ;[1 1 1] Follow after take damage
  (EventDispatchers|BindEventtoOnTakeAnyDamage (Game|GetInstigator) (delegate Custom|TakeDamage)))

(fn ConstructionScript)